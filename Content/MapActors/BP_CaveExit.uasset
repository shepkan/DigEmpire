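; BP_CaveExit is a map actor that gates the player's passage deeper into the cave behind a gold requirement.
; When the local player's character enters its sphere, it reads the gold ore amount from the player controller's inventory and compares it to GoldThreshold.
; With enough gold, it shows an approving HUD message and opens L_Cave after a short delay, without deducting gold; otherwise the message states the required amount.
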(event OnComponentBeginOverlap(Sphere)
  (params (OverlappedComponent :type Primitive%20Component%20Object%20Reference) (OtherActor :type Actor%20Object%20Reference) (OtherComp :type Primitive%20Component%20Object%20Reference) (OtherBodyIndex :type Integer) (bFromSweep :type Boolean) (SweepResult :type Hit%20Result%20Structure%20%28by%20ref%29))
  (bind _returnvalue (Game|GetPlayerController 0))
  (bind _asbp_base_character (Utilities|Casting|CastToBP_BaseCharacter OtherActor))
  (if (== (Pawn|GetController _asbp_base_character) _returnvalue)
    (bind _asdig_empire_player_controller (Utilities|Casting|CastToDigEmpirePlayerController _returnvalue))
    (if (>= (Class|DEInventoryComponent|GetResourceAmount (Class|DigEmpirePlayerController|GetInventory _asdig_empire_player_controller) (GameplayTags|MakeLiteralGameplayTag "(TagName=\"Gameplay.Ore.Gold\")")) (Variables|Default|GetGoldThreshold))
      (Default|PlayerMessage (Variables|/Game/Character/BP_BaseCharacter.BP_BaseCharacter_C|GetPlayer%20HUD _asbp_base_character) (Utilities|Text|ToText(String) (Utilities|String|MakeLiteralString "Hmm... Ok, ypu can go deeper.")))
      (Utilities|FlowControl|Delay 3.0)
      (Game|OpenLevel(byObjectReference) "/Game/Map/L_Cave.L_Cave")
      (else
        (Default|PlayerMessage (Variables|/Game/Character/BP_BaseCharacter.BP_BaseCharacter_C|GetPlayer%20HUD _asbp_base_character) (Utilities|Text|ToText(String) (Utilities|String|Append (Utilities|String|MakeLiteralString "Who are you? You are not welcome here. Bring ") (Utilities|String|ToString(Integer) (Variables|Default|GetGoldThreshold)) (Utilities|String|MakeLiteralString " and we will consider your status."))))))))

(event EventBeginPlay)

(event Collision|EventActorBeginOverlap
  (params (OtherActor :type Actor%20Object%20Reference)))

(event EventTick
  (params (DeltaSeconds :type Float%20%28single-precision%29)))

(fn ConstructionScript)